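; SplineWall is a structure Blueprint that builds a wall from spline mesh components in its Construction Script.
; It adds one spline mesh component per segment between consecutive spline points and calls AttachComponentToComponent with KeepRelative rules.
; The SetStartAndEnd node that would fit each mesh to its segment's local locations and tangents is never executed, so segments are not shaped to the spline.
; The event graph holds only disabled placeholder events.
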(event EventBeginPlay)

(event Collision|EventActorBeginOverlap
  (params (OtherActor :type Actor%20Object%20Reference)))

(event EventTick
  (params (DeltaSeconds :type Float%20%28single-precision%29)))

(fn ConstructionScript
  (|CallParentFunction)
  (for _index (range 0 (- (Spline|GetNumberOfSplinePoints (Variables|Default|GetSpline)) 2))
    (bind _returnvalue (AddComponent|AddSplineMeshComponent false))
    (Transformation|AttachComponentToComponent _returnvalue 0 "None" "KeepRelative" "KeepRelative" "KeepRelative" true)))