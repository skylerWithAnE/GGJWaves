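; BP_Pawn is an enemy Blueprint that deals repeated damage to its attack target, extending a parent class's behavior.
; On AttackTick it runs the parent logic, then applies damage to a valid AttackTarget through a DoOnce gate.
; A retriggerable delay resets the gate after the attack rate, shortened by a few frames' worth of delta time.
; BeginPlay, Tick and construction only call the parent.
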(event EventBeginPlay
  (|CallParentFunction))

(event EventTick
  (params (DeltaSeconds :type Float%20%28single-precision%29))
  (|CallParentFunction DeltaSeconds))

(event EventAttackTick
  (|CallParentFunction)
  (bind _attack_target (Variables|Default|GetAttack%20Target)
    (:then
      (Utilities|FlowControl|DoOnce false :!label _label
        (:Completed
          (Game|Damage|ApplyDamage _attack_target (Variables|Default|GetdamageVal) 0 0)
          (Utilities|FlowControl|RetriggerableDelay (- (Variables|Default|GetAttack%20Rate) (* (Utilities|Time|GetWorldDeltaSeconds) 5.0)))
          (goto _label Reset))))
    (:else)))

(fn ConstructionScript
  (|CallParentFunction))