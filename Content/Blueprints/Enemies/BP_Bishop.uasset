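; BP_Bishop is a ranged enemy that fires projectiles at its target, built on a parent class whose events it extends.
; On each AttackTick, after the parent logic, it spawns a BP_EnemyProjectile at ShotOrigin regardless of collision.
; The shot's rotation points from the actor's location, rather than ShotOrigin, toward the target.
; Tick switches on CurrentActivity after the parent call, but no branch has logic.
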(event EventTick
  (params (DeltaSeconds :type Float%20%28single-precision%29))
  (|CallParentFunction DeltaSeconds)
  (switch Utilities|FlowControl|Switch|SwitchonEnum_PieceActivity (Variables|Default|GetCurrent%20Activity)))

(event EventBeginPlay
  (|CallParentFunction))

(event EventAttackTick
  (|CallParentFunction)
  (Game|SpawnActorfromClass "/Game/Blueprints/Weapons/Projectiles/BP_EnemyProjectile.BP_EnemyProjectile_C" (Math|Transform|MakeTransform (Transformation|GetWorldLocation (Variables|Default|GetShotOrigin)) (Math|Rotator|FindLookatRotation (Transformation|GetActorLocation) (Transformation|GetActorLocation (CallFunction|GetTarget)))) "AlwaysSpawn" 0 0))

(fn ConstructionScript
  (|CallParentFunction))