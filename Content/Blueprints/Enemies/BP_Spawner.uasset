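; BP_Spawner is an enemy spawner that tops up enemies at the level's BP_SpawnPoint actors while EnemyCount is below EnemyCap.
; BeginPlay gathers the spawn points and shuffles EnemySpawnList.
; Each Tick below the cap asks a random point to spawn the next list entry, advancing only on success.
; The index wraps and reshuffles at the spawn point count, not the list length, and EnemyCount is not updated here.
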(event EventBeginPlay
  (bind _outactors (Actor|GetAllActorsOfClass "/Game/Blueprints/Enemies/BP_SpawnPoint.BP_SpawnPoint_C"))
  (Variables|Default|SetSpawnPoints _outactors)
  (Utilities|Array|Shuffle (Variables|Default|GetEnemySpawnList)))

(event EventTick
  (params (DeltaSeconds :type Float%20%28single-precision%29))
  (bind _spawnpoints (Variables|Default|GetSpawnPoints))
  (bind _returnvalue (Utilities|Array|Length _spawnpoints))
  (if (< (Variables|Default|GetEnemy%20Count) (Variables|Default|GetEnemy%20Cap))
    (bind _newparam (Default|SpawnEnemy (Utilities|Array|Get(acopy) _spawnpoints (Math|Random|RandomInteger _returnvalue)) (Utilities|Array|Get(acopy) (Variables|Default|GetEnemySpawnList) (Variables|Default|GetSpawn%20Index))))
    (if _newparam
      (bind _result (Math|Integer|IncrementInt (Variables|Default|GetSpawn%20Index))
        (:%20%20
          (if (== _result _returnvalue)
            (Variables|Default|SetSpawn%20Index 0)
            (Utilities|Array|Shuffle (Variables|Default|GetEnemySpawnList))))))))

(fn ConstructionScript)