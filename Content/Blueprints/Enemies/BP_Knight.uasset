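; Knight enemy that performs a jump attack when the main character enters its damage collider.
; On overlap it stops, disables gravity and builds attack points from offsets and the target's location.
; A looping timer interpolates it along those points, with logic to restore gravity and launch it at the target.
; The End Attack tick handles knockback damage to nearby pawns, while an AttackTick override applies direct damage in range.
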(event OnComponentBeginOverlap(DamageCollider)
  (params (OverlappedComponent :type Primitive%20Component%20Object%20Reference) (OtherActor :type Actor%20Object%20Reference) (OtherComp :type Primitive%20Component%20Object%20Reference) (OtherBodyIndex :type Integer) (bFromSweep :type Boolean) (SweepResult :type Hit%20Result%20Structure%20%28by%20ref%29))
  (bind _asbp_main_character (Utilities|Casting|CastToBP_MainCharacter OtherActor))
  (switch Utilities|FlowControl|Switch|SwitchonEnum_PieceActivity (Variables|Default|GetCurrent%20Activity)
    (:NewEnumerator0
      (Variables|Default|SetCurrent%20Activity "NewEnumerator1"))
    (:NewEnumerator1
      _))
  (Utilities|FlowControl|DoOnce false
    (:Completed
      (Variables|Default|SetAttack%20Target _asbp_main_character)
      (CallFunction|SetAttackVectors)
      (Variables|Default|SetMove%20Point%20Index 0)
      (Components|Movement|StopMovementImmediately (Variables|Character|GetCharacterMovement))
      (Utilities|Time|SetTimerbyEvent (delegate Custom|AttackMovement) 0.033 true))))

(event OnComponentEndOverlap(DamageCollider)
  (params (OverlappedComponent :type Primitive%20Component%20Object%20Reference) (OtherActor :type Actor%20Object%20Reference) (OtherComp :type Primitive%20Component%20Object%20Reference) (OtherBodyIndex :type Integer))
  (Utilities|Casting|CastToBP_MainCharacter OtherActor)
  (switch Utilities|FlowControl|Switch|SwitchonEnum_PieceActivity (Variables|Default|GetCurrent%20Activity)
    (:NewEnumerator2
      (Variables|Default|SetCurrent%20Activity "NewEnumerator0"))))

(event Custom|Complete%20Attack
  (CallFunction|KnockAround (Transformation|GetActorLocation) 4e+02 (Utilities|Array|MakeArray "ObjectTypeQuery3") 2.0 (Variables|Default|GetKnock%20Around%20Impulse) (Variables|Default|GetJumpAttackDamage) self)
  (Utilities|FlowControl|DoOnce false) ; enters at Reset
)

(event Custom|AttackMovement
  (bind _returnvalue (Transformation|GetActorLocation))
  (if (Math|Vector|Equal(Vector) (Utilities|Array|Get(acopy) (Variables|Default|GetAttack%20Vectors) (Variables|Default|GetMove%20Point%20Index)) _returnvalue 1.0)
    (Math|Integer|IncrementInt (Variables|Default|GetMove%20Point%20Index)
      (:%20%20
        (if (== (Variables|Default|GetMove%20Point%20Index) 0)
          (Utilities|Time|SetTimerbyEvent (delegate Custom|AttackMovement) 0.0)
          (Utilities|FlowControl|Delay 0.025)
          (Variables|/Script/Engine.CharacterMovementComponent|SetGravityScale (Variables|Character|GetCharacterMovement) 1.0)
          (Physics|AddImpulse (Variables|Character|GetCharacterMovement) (* (Math|Vector|GetUnitDirection(Vector) (Transformation|GetActorLocation) (Utilities|Array|Get(acopy) (Variables|Default|GetAttack%20Vectors) 2)) 2e+03) true)
          (Variables|Default|SetCurrent%20Activity "NewEnumerator2")
          (Variables|Default|SetMove%20Point%20Index 0))))
    (else
      (Transformation|SetActorLocation (Math|Interpolation|VInterpTo _returnvalue (Utilities|Array|Get(acopy) (Variables|Default|GetAttack%20Vectors) (Variables|Default|GetMove%20Point%20Index)) 0.033 15.0) true false))))

(event EventBeginPlay
  (|CallParentFunction))

(event EventAttackTick
  (bind _attack_target (Variables|Default|GetAttack%20Target))
  (switch Utilities|FlowControl|Switch|SwitchonEnum_PieceActivity (Variables|Default|GetCurrent%20Activity)
    (:NewEnumerator0
      _)
    (:NewEnumerator2
      _))
  (if (>= (Transformation|GetDistanceTo _attack_target self) (Variables|Default|GetAutoAttackRange))
    (Variables|Default|SetCurrent%20Activity "NewEnumerator0")
    (else
      (Game|Damage|ApplyDamage _attack_target (Variables|Default|GetdamageVal) 0 0))))

(event EventTick
  (params (DeltaSeconds :type Float%20%28single-precision%29))
  (|CallParentFunction DeltaSeconds)
  (switch Utilities|FlowControl|Switch|SwitchonEnum_PieceActivity (Variables|Default|GetCurrent%20Activity)
    (:NewEnumerator2
      (if (AI|Components|NavMovement|IsFalling (Variables|Character|GetCharacterMovement))
        (goto _label Reset)
        (else
          (Utilities|FlowControl|Sequence
            (:then_0
              (Utilities|FlowControl|DoOnce false :!label _label
                (:Completed
                  (CallFunction|CompleteAttack))))
            (:then_1
              (CallFunction|MoveEvent))))))))

(fn ConstructionScript
  (|CallParentFunction))

(fn SetAttackVectors
  (bind _attack_vector_offset (Variables|Default|GetAttack%20Vector%20Offset))
  (bind _attack_vectors (Variables|Default|GetAttack%20Vectors))
  (bind _attack_target (Variables|Default|GetAttack%20Target))
  (Utilities|Array|SetArrayElem _attack_vectors 0 (+ (Transformation|GetActorLocation) _attack_vector_offset) true)
  (Utilities|Array|SetArrayElem _attack_vectors 1 (* (+ (Utilities|Array|Get(acopy) _attack_vectors) (+ (Transformation|GetActorLocation _attack_target) _attack_vector_offset)) 0.45) true)
  (Utilities|Array|SetArrayElem _attack_vectors 2 (Transformation|GetActorLocation _attack_target))
  (Variables|/Script/Engine.CharacterMovementComponent|SetGravityScale (Variables|Character|GetCharacterMovement) 0.0)
  (Variables|Default|SetDo%20Attack true))