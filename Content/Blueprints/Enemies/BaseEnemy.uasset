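; Base enemy that chases the player and deals repeated contact damage to BP_MainCharacter.
; On BeginPlay it spawns its default controller, then reissues SimpleMoveToActor toward the player pawn every Tick.
; DamageCollider overlap starts a one-second looping timer with an immediate first hit of DamageVal.
; Each pulse checks Sphere overlaps, clearing the timer through a zero-time SetTimerByEvent once the character is gone.
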(event OnComponentBeginOverlap(DamageCollider)
  (params (OverlappedComponent :type Primitive%20Component%20Object%20Reference) (OtherActor :type Actor%20Object%20Reference) (OtherComp :type Primitive%20Component%20Object%20Reference) (OtherBodyIndex :type Integer) (bFromSweep :type Boolean) (SweepResult :type Hit%20Result%20Structure%20%28by%20ref%29))
  (Utilities|Casting|CastToBP_MainCharacter OtherActor)
  (if (not (Utilities|Time|IsValidTimerHandle (Variables|Default|Gettimer)))
    (bind _returnvalue (Utilities|Time|SetTimerbyEvent (delegate Custom|damageWhileInRadius) 1.0 true))
    (CallFunction|DamageWhileinRadius)
    (bind _output_get (Variables|Default|Settimer _returnvalue))))

(event Custom|damageWhileInRadius
  (bind _sphere (Variables|Default|GetSphere))
  (bind _overlappingactors (Collision|GetOverlappingActors _sphere "/Game/Blueprints/BP_MainCharacter.BP_MainCharacter_C" :!class /Script/Engine.PrimitiveComponent))
  (bind _item (Utilities|Array|Get(acopy) _overlappingactors))
  (Development|PrintString "boop")
  (Utilities|IsValid _item
    (:Is%20Valid
      (Game|Damage|ApplyDamage _item (Variables|Default|GetdamageVal) 0 self))
    (:Is%20Not%20Valid
      (Utilities|Time|SetTimerbyEvent (delegate Custom|damageWhileInRadius) 0.0)
      (Variables|Default|Settimer ""))))

(event EventBeginPlay
  (Pawn|SpawnDefaultController))

(event EventTick
  (params (DeltaSeconds :type Float%20%28single-precision%29))
  (AI|Navigation|SimpleMovetoActor (Pawn|GetController) (Game|Player|GetPlayerPawn 0)))

(fn ConstructionScript)