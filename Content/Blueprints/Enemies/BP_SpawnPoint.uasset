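; Enemy spawn point Blueprint that spawns enemy actors inside a box volume and keeps track of them.
; SpawnEnemy spawns the given class at a random point in the box's bounds, always spawning regardless of collision, records it in SpawnedEnemies and returns whether it succeeded.
; Each Tick it loops over that array and removes entries that are no longer valid.
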(event EventTick
  (params (DeltaSeconds :type Float%20%28single-precision%29))
  (bind _spawned_enemies (Variables|Default|GetSpawned%20Enemies))
  (for _array_element _spawned_enemies
    (Utilities|IsValid _array_element
      (:Is%20Not%20Valid
        (Utilities|Array|RemoveItem _spawned_enemies _array_element)))))

(fn ConstructionScript)

(fn SpawnEnemy
  (params (Class :type Base%20Enemy%20Class%20Reference))
  (bind _box (Variables|Default|GetBox))
  (bind _returnvalue (Game|SpawnActorfromClass Class (Math|Conversions|ToTransform(Vector) (Math|Random|RandomPointinBoundingBox (Transformation|GetWorldLocation _box) (Variables|/Script/Engine.BoxComponent|GetBoxExtent _box))) "AlwaysSpawn" 0 0))
  (Utilities|IsValid _returnvalue
    (:Is%20Valid
      (Utilities|Array|Add (Variables|Default|GetSpawned%20Enemies) _returnvalue)
      (return true))
    (:Is%20Not%20Valid
      (return false))))