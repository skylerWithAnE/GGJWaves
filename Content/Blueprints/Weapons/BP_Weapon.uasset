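; Pickup weapon actor that can be highlighted, collected by a holder and fired at a target location.
; Focus toggles custom depth on the static mesh with a fixed stencil value for highlighting.
; Pickup stores the collector as Holder, disables sphere collision and sends the unfocus message.
; Attack spawns the configurable ShotClass at ShotOrigin, rotated toward the target; PickedUp and EndAttack are empty.
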(event Custom|Attack
  (params (Target :type Vector))
  (bind _shotorigin (Variables|Default|GetShotOrigin))
  (bind _returnvalue (Transformation|GetWorldLocation _shotorigin))
  (Game|SpawnActorfromClass (Variables|Default|GetShotClass) (Math|Transform|MakeTransform _returnvalue (Math|Rotator|FindLookatRotation _returnvalue Target)) "AdjustIfPossibleButAlwaysSpawn" 0 0))

(event Custom|Picked%20Up
  (params (Collector :type BP%20Main%20Character%20Object%20Reference)))

(event Custom|EndAttack)

(event EventGetPickedUp
  (params (Collector :type BP%20Main%20Character%20Object%20Reference))
  (Variables|Default|SetHolder Collector)
  (Collision|SetCollisionEnabled (Variables|Default|GetSphere) "NoCollision")
  (Class|BPIPickup|Focus(Message) self true))

(event EventFocus
  (params (Unfocus :type Boolean))
  (bind _staticmesh (Variables|Default|GetStaticMesh))
  (Rendering|SetRenderCustomDepth _staticmesh (not Unfocus))
  (Rendering|SetCustomDepthStencilValue _staticmesh 253))

(fn ConstructionScript)